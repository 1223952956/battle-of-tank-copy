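; BP_GM_Lobby is the waiting-room game mode for Battle of Tanks, maintaining the lobby's player list.
; It caches RoomInfo from the game instance at BeginPlay and collects controllers on PostLogin.
; Events add player info or replace entries by name, with changes triggering team and list refreshes.
; Refreshes loop over each BP_WaitRoomController, passing the list, with the player-list update adding a team or melee label from the room type.
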(event `self.ReceiveBeginPlay`
  ;[1 1 1] 保存房间信息
  (bind _asbp_battle_of_tanks_game_instance (cast `/Game/Blueprint/BP_BattleOfTanksGameInstance` (`GameplayStatics.GetGameInstance`)))
  (set `self.Room Info` (`/Game/Blueprint/BP_BattleOfTanksGameInstance.RoomInfo` _asbp_battle_of_tanks_game_instance)))

(event `self.K2_PostLogin`
  (params (NewPlayer :type "PlayerController Object Reference"))
  ;[1 1 1] 玩家登录
  (`KismetArrayLibrary.Array_Add` (`self.Player Controllers`) NewPlayer))

(event `Event_UpdateListMulticast`
  (bind _playerinfolist (`self.PlayerInfoList`))
  ;[1 1 1] 更新所有玩家列表
  (for _array_element (`self.Player Controllers`)
    (bind _asbp_wait_room_controller (cast `/Game/Blueprint/BP_WaitRoomController` _array_element))
    (switch `/Game/Blueprint/ERoomType` (`.RoomType_6_F1FE08B041187209279150A14384B472` (break `/Game/Blueprint/FRoomInfo` (`self.Room Info`)))
      (:`NewEnumerator0`
        (`/Game/Blueprint/BP_WaitRoomController.Event_UpdateList` _asbp_wait_room_controller _playerinfolist "组队"))
      (:`NewEnumerator1`
        (`/Game/Blueprint/BP_WaitRoomController.Event_UpdateList` _asbp_wait_room_controller _playerinfolist "混战")))))

(event `Event_AddPlayerInfo`
  (params (NewItem :type "/Game/Blueprint/FPlayerInfo Structure (by ref)"))
  ;[1 1 1] 添加玩家信息
  (`KismetArrayLibrary.Array_Add` (`self.PlayerInfoList`) NewItem))

(event `Event_ChangePlayerInfo`
  (params (InPlayerInfo :type "/Game/Blueprint/FPlayerInfo Structure"))
  (bind _playerinfolist (`self.PlayerInfoList`))
  ;[1 1 1] 更改指定玩家信息
  (for (_array_element _array_index) (`self.PlayerInfoList`)
    (if (`KismetStringLibrary.EqualEqual_StrStr` (`.PlayerName_5_55C07394411E9584ACE13CBE79BECD37` (break `/Game/Blueprint/FPlayerInfo` _array_element)) (`.PlayerName_5_55C07394411E9584ACE13CBE79BECD37` (break `/Game/Blueprint/FPlayerInfo` InPlayerInfo)))
      (`KismetArrayLibrary.Array_Remove` _playerinfolist _array_index)
      (`KismetArrayLibrary.Array_Add` _playerinfolist InPlayerInfo)))
  (`self.Event_UpdatePlayerTeamList`)
  (`self.Event_UpdateListMulticast`))

(event `Event_UpdatePlayerTeamList`
  ;[1 1 1] 更新所有玩家组队信息
  (for _array_element (`self.Player Controllers`)
    (bind _asbp_wait_room_controller (cast `/Game/Blueprint/BP_WaitRoomController` _array_element))
    (`/Game/Blueprint/BP_WaitRoomController.Event_UpdateTeamList` _asbp_wait_room_controller (`self.PlayerInfoList`))))

(fn `UserConstructionScript`)