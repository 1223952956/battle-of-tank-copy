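; Player controller for the tank battle game that spawns each player's team tank and shows the win screen.
; On local BeginPlay it passes the GameInstance's player info to SetPlayerInfoServer, which stores it and asks the GameMode to start spawning.
; StartPlayerPawn replaces any existing pawn with a possessed, team-colored BP_Tank at a tag-matched PlayerStart, destroying that start afterward.
; DisplayWinUI swaps all widgets for BP_WinUI and shows the cursor.
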(event `self.ReceiveBeginPlay`
  (if (`self.IsLocalPlayerController`)
    (bind _asbp_battle_of_tanks_game_instance (cast `/Game/Blueprint/BP_BattleOfTanksGameInstance` (`GameplayStatics.GetGameInstance`)))
    (`self.SetPlayerInfoServer` (`/Game/Blueprint/BP_BattleOfTanksGameInstance.PlayerInfo` _asbp_battle_of_tanks_game_instance))))

(event `SetPlayerInfoServer`
  (params (InPlayerInfo :type "/Game/Blueprint/FPlayerInfo Structure"))
  (set `self.CtrlPlayerInfo` InPlayerInfo)
  (bind _asbp_battle_of_tanks_game_mode_base (cast `/Game/Blueprint/BP_BattleOfTanksGameModeBase` (`GameplayStatics.GetGameMode`)))
  (`/Game/Blueprint/BP_BattleOfTanksGameModeBase.StartSpawnPawn` _asbp_battle_of_tanks_game_mode_base self))

(event `StartPlayerPawn`
  (bind _returnvalue (`self.K2_GetPawn`))
  ;[1 1 1] 根据队伍设置出生点标签
  (if (!= _returnvalue null)
    (`self.K2_DestroyActor` _returnvalue))
  (switch `/Game/Blueprint/ETeamType` (`.PlayerTeam_9_1E4E64F1478A3740B217499DEC73A146` (break `/Game/Blueprint/FPlayerInfo` (`self.CtrlPlayerInfo`)))
    (:`NewEnumerator0`
      _)
    (:`NewEnumerator1`
      (set `self.PawnSpawnTag` "RedTeam"))
    (:`NewEnumerator2`
      (set `self.PawnSpawnTag` "BlueTeam")))
  (`self.FindStartLocation`))

(event `FindStartLocation`
  ;[1 1 1] 根据出生点标签选择出生点
  (bind _outactors (`GameplayStatics.GetAllActorsOfClass` "/Script/Engine.PlayerStart"))
  (for _array_element _outactors
    (if (== (`PlayerStart.PlayerStartTag` _array_element) (`self.PawnSpawnTag`))
      (`self.SpawnPawn` (`self.GetTransform` _array_element))
      (`self.K2_DestroyActor` _array_element)
      (break))))

(event `SpawnPawn`
  (params (Transform :type "Transform Structure"))
  (bind _ownpawn (`self.OwnPawn`))
  ;[1 1 1] 生成pawn
  (bind _returnvalue (`|SpawnActorFromClass` "/Game/Tank/BP_Tank.BP_Tank_C" Transform "AdjustIfPossibleButAlwaysSpawn" "OverrideRootScale" null null))
  (bind _output_get (set `self.OwnPawn` _returnvalue))
  (`self.Possess` _output_get)
  (`/Game/Tank/BP_Tank.SetHPBarVisibility` _output_get)
  (`/Game/Tank/BP_Tank.CreatePlayerWidget` _output_get)
  (switch `/Game/Blueprint/ETeamType` (`.PlayerTeam_9_1E4E64F1478A3740B217499DEC73A146` (break `/Game/Blueprint/FPlayerInfo` (`self.CtrlPlayerInfo`)))
    (:`NewEnumerator0`
      (set `Tank.CampFlag` 0 _ownpawn))
    (:`NewEnumerator1`
      (set `Tank.CampFlag` 1 _ownpawn))
    (:`NewEnumerator2`
      (set `Tank.CampFlag` 2 _ownpawn)))
  (`/Game/Tank/BP_Tank.SetColorByTeam` (`self.OwnPawn`)))

(event `DisplayWinUI`
  ;[1 1 1] 显示胜利UI
  (`WidgetLayoutLibrary.RemoveAllWidgets`)
  (bind _returnvalue (`|CreateWidget` "/Game/UI/BP_WinUI.BP_WinUI_C" self))
  (`UserWidget.AddToViewport` _returnvalue 0)
  (set `self.bShowMouseCursor` true))

(fn `UserConstructionScript`)