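; AI tank Blueprint that wires up its barrel, turret, camera gimbal and health bar widget, and tints itself by team.
; On BeginPlay it passes component references to setup functions, links the HP bar to itself and picks the body material from CampFlag.
; Helper events create the player UI and hide the floating HP bar when player 0 controls the tank.
; On destruction it tells the game mode to reduce the AI tank count.
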(event `self.ReceiveBeginPlay`
  (`self.SetBarrelAndTurretReference` (`self.Barrel`) (`self.Turret`))
  (`self.SetCameraReference` (`self.Azimuth Gimbal`) (`self.SpringArm`))
  (bind _asbp_hpbar (cast `/Game/UI/BP_HPBar` (`WidgetComponent.GetWidget` (`self.Widget`))))
  (set `/Game/UI/BP_HPBar.OwnerTank` self _asbp_hpbar)
  (`self.SetColorByTeam`))

(event `CreatePlayerWidget`
  (bind _returnvalue (`|CreateWidget` "/Game/UI/BP_PlayerUI.BP_PlayerUI_C" (`GameplayStatics.GetPlayerController` 0)))
  (`UserWidget.AddToViewport` _returnvalue 0))

(event `SetHPBarVisibility`
  ;[1 1 1] 设定跟随血条的显示
  (`SceneComponent.SetVisibility` (`self.Widget`) (!= (`self.GetController`) (`GameplayStatics.GetPlayerController` 0)) false))

(event `SetColorByTeam`
  (bind _tank (`self.Tank`))
  ;[1 1 1] 更改颜色显示
  (switch `int` (`self.CampFlag`)
    (:`0`
      (`PrimitiveComponent.SetMaterial` _tank 0 null))
    (:`1`
      (`PrimitiveComponent.SetMaterial` _tank 0 "/Game/StarterContent/Materials/M_Water_Ocean.M_Water_Ocean"))
    (:`2`
      (`PrimitiveComponent.SetMaterial` _tank 0 "/Game/StarterContent/Materials/M_Wood_Pine.M_Wood_Pine"))))

(event `self.ReceiveDestroyed`
  ;[1 1 1] 销毁事件
  (bind _asbp_battle_of_tanks_game_mode_base (cast `/Game/Blueprint/BP_BattleOfTanksGameModeBase` (`GameplayStatics.GetGameMode`)))
  (`/Game/Blueprint/BP_BattleOfTanksGameModeBase.ReducecAITankNum` _asbp_battle_of_tanks_game_mode_base))

(fn `UpdateMoveSpeed`
  (params (NewMoveSpeed :type "Float (double-precision)"))
  (set `self.MaxMoveSpeed` NewMoveSpeed))

(fn `UserConstructionScript`)