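; Tank Blueprint for a team-based tank battle, handling component setup, team coloring and player UI.
; BeginPlay passes barrel, turret and camera components to setters, links the HP bar widget to itself and picks a material by CampFlag.
; Display events forward shield slot, storage and reload feedback to the player widget, and the HP bar hides for the local player.
; Defeat events show the defeat screen and remove the controller through the game mode.
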(event `self.ReceiveBeginPlay`
  ;[1 1 1] 初始化
  (`self.SetBarrelAndTurretReference` (`self.Barrel`) (`self.Turret`))
  (`self.SetCameraReference` (`self.Azimuth Gimbal`) (`self.SpringArm`))
  (bind _asbp_hpbar (cast `/Game/UI/BP_HPBar` (`WidgetComponent.GetWidget` (`self.Widget`))))
  (set `/Game/UI/BP_HPBar.OwnerTank` self _asbp_hpbar)
  (`self.SetColorByTeam`))

(event `CreatePlayerWidget`
  ;[1 1 1] 创建玩家UI
  (bind _returnvalue (`|CreateWidget` "/Game/UI/BP_PlayerUI.BP_PlayerUI_C" (`GameplayStatics.GetPlayerController` 0)))
  (`UserWidget.AddToViewport` _returnvalue 0)
  (set `self.FocusedWidget` _returnvalue))

(event `SetHPBarVisibility`
  ;[1 1 1] 设定跟随血条的显示
  (`SceneComponent.SetVisibility` (`self.Widget`) (!= (`self.GetController`) (`GameplayStatics.GetPlayerController` 0)) false))

(event `SetColorByTeam`
  (bind _tank (`self.Tank`))
  ;[1 1 1] 更改颜色显示
  (switch `int` (`self.CampFlag`)
    (:`0`
      (`PrimitiveComponent.SetMaterial` _tank 0 null))
    (:`1`
      (`PrimitiveComponent.SetMaterial` _tank 0 "/Game/StarterContent/Materials/M_Water_Ocean.M_Water_Ocean"))
    (:`2`
      (`PrimitiveComponent.SetMaterial` _tank 0 "/Game/StarterContent/Materials/M_Wood_Pine.M_Wood_Pine"))))

(event `self.ReceiveDestroyed`
  ;[1 1 1] 废弃
)

(event `RemoveControllerServer`
  (params (InPlayerController :type "PlayerController Object Reference"))
  ;[1 1 1] 废弃
  (bind _asbp_tank_player_controller (cast `/Game/Blueprint/BP_TankPlayerController` InPlayerController))
  (bind _asbp_battle_of_tanks_game_mode_base (cast `/Game/Blueprint/BP_BattleOfTanksGameModeBase` (`GameplayStatics.GetGameMode`)))
  (`/Game/Blueprint/BP_BattleOfTanksGameModeBase.RemoveController` _asbp_battle_of_tanks_game_mode_base _asbp_tank_player_controller))

(event `self.DisplayDefeatUI`
  (bind _returnvalue (`GameplayStatics.GetPlayerController` 0))
  ;[1 1 1] 失败UI显示
  (`WidgetLayoutLibrary.RemoveAllWidgets`)
  (bind _astank_player_controller (cast `TankPlayerController` _returnvalue))
  (bind _returnvalue_2 (`|CreateWidget` "/Game/UI/BP_DefeatUI.BP_DefeatUI_C" _astank_player_controller))
  (`UserWidget.AddToViewport` _returnvalue_2 0)
  (set `PlayerController.bShowMouseCursor` true _returnvalue))

(event `self.RemoveController`
  ;[1 1 1] 告知服务器 玩家已失败
  (bind _asbp_battle_of_tanks_game_mode_base (cast `/Game/Blueprint/BP_BattleOfTanksGameModeBase` (`GameplayStatics.GetGameMode`)))
  (bind _asbp_tank_player_controller (cast `/Game/Blueprint/BP_TankPlayerController` (`self.GetController`)))
  (`/Game/Blueprint/BP_BattleOfTanksGameModeBase.RemoveController` _asbp_battle_of_tanks_game_mode_base _asbp_tank_player_controller))

(event `self.DisplaySelectedSlot`
  (params (InSlotIndex :type Integer))
  ;[1 1 1] 显示被选择的护盾插槽
  (`/Game/UI/BP_PlayerUI.HighLightShieldSlot` (`self.FocusedWidget`) InSlotIndex))

(event `self.DisplayShieldStorage`
  ;[1 1 1] 显示护盾仓库
  (`/Game/UI/BP_PlayerUI.UpdateShieldStorage` (`self.FocusedWidget`)))

(event `self.DisplaySelectedStorage`
  ;[1 1 1] 显示被选中的仓库格子
  (`/Game/UI/BP_PlayerUI.HighlightShieldStoraged` (`self.FocusedWidget`)))

(event `self.DisplayLoadCannon`
  ;[1 1 1] 显示装弹动画
  (`/Game/UI/BP_PlayerUI.LoadCannon` (`self.FocusedWidget`)))

(fn `UpdateMoveSpeed`
  (params (NewMoveSpeed :type "Float (double-precision)"))
  (set `self.MaxMoveSpeed` NewMoveSpeed))

(fn `UserConstructionScript`)